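; BP_ModManager is the Mercury mod manager, bridging C++-hooked functions and the mod manager UI for updates, downloads and load order.
; On BeginPlay it triggers an update check and scans the asset registry for ModSettings data assets.
; Tick refreshes the outdated-mod notifier and finds the ModStack widget, linking itself to it.
; Helper functions fill that widget's pak lists, read back load order and push download progress, while empty functions serve as hook points.
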(event EventBeginPlay
  (Utilities|FlowControl|Delay 0.5)
  (DownloadManager|CheckforUpdates)
  (ModSettings|GetModSettingsDA))

(event EventTick
  (params (DeltaSeconds :type Float%20%28single-precision%29))
  (Utilities|FlowControl|Sequence
    (:then_0
      (if (not (Utilities|Enum|Equal(Enum) (Class|RichTextBlock|GetText (Variables|/Game/Mods/Mercury/UI/Widgets/WBP_UI_ModManager_MainMenuNotifier.WBP_UI_ModManager_MainMenuNotifier_C|GetUpdatesCountText (Variables|Default|GetModManagerNotifier))) (Utilities|Text|ToText(Integer) (Variables|DownloadManager|GetOutdatedMods))))
        (DownloadManager|UpdateOutdatedModCount)))
    (:then_1
      (Variables|Default|GetModStack
        (:then)
        (:else
          (bind _foundwidgets (Widget|GetAllWidgetsOfClass "/Game/Mods/Mercury/UI/Widgets/WBP_UI_ModManager_ModStack.WBP_UI_ModManager_ModStack_C" false))
          (for _array_element _foundwidgets
            (bind _output_get (Variables|Default|SetModStack _array_element))
            (Variables|/Game/Mods/Mercury/UI/Widgets/WBP_UI_ModManager_ModStack.WBP_UI_ModManager_ModStack_C|SetModManager _output_get self)
            (Variables|Default|SetHasModStack true)))))))

(fn ConstructionScript
  (|CallParentFunction))

(fn CheckforUpdates
  ;[1 1 1] Hooked into in c++
)

(fn UpdateOutdatedModCount
  (bind _outdatedmods (Variables|DownloadManager|GetOutdatedMods))
  (Default|UpdateModText (Variables|Default|GetModManagerNotifier) (Utilities|Text|ToText(Integer) _outdatedmods) _outdatedmods))

(fn AddPaktoLoadOrderList
  (params (PakName :type String))
  (Default|AddPaktoContainer (Variables|/Game/Mods/Mercury/UI/Widgets/WBP_UI_ModManager_ModStack.WBP_UI_ModManager_ModStack_C|GetWBP_UI_ModManager_LoadOrder (Variables|Default|GetModStack)) (Utilities|Text|ToText(String) PakName)))

(fn RefreshLoadOrder
  ;[1 1 1] Hooked in c++
)

(fn GetandSetLoadOrderPakStringsArray
  (bind _modstack (Variables|Default|GetModStack)
    (:then
      (Utilities|Array|Clear (Variables|LoadOrder|GetLoadOrderPakStrings))
      (for _array_element (Class|PanelWidget|GetAllChildren (Variables|/Game/Mods/Mercury/UI/Widgets/LoadOrder/WBP_UI_ModManager_LoadOrder.WBP_UI_ModManager_LoadOrder_C|GetPakModsContainer (Variables|/Game/Mods/Mercury/UI/Widgets/WBP_UI_ModManager_ModStack.WBP_UI_ModManager_ModStack_C|GetWBP_UI_ModManager_LoadOrder _modstack)))
        (bind _aswbp_ui_mod_manager_base_pak_mod (Utilities|Casting|CastToWBP_UI_ModManager_BASE_PakMod _array_element))
        (Utilities|Array|AddUnique (Variables|LoadOrder|GetLoadOrderPakStrings) (Utilities|String|ToString(Text) (Class|TextBlock|GetText (Variables|/Game/Mods/Mercury/UI/Widgets/LoadOrder/WBP_UI_ModManager_BASE_PakMod.WBP_UI_ModManager_BASE_PakMod_C|GetText_ModName_1 _aswbp_ui_mod_manager_base_pak_mod))))))
    (:else)))

(fn UpdatePakMod
  (params (PakName :type String))
  ;[1 1 1] Hooked in C++
)

(fn GetModSettingsDA
  (bind _filter (LocalVariables|GetFilter))
  (Class|AssetRegistry|ScanPathsSynchronous (Class|AssetRegistryHelpers|GetAssetRegistry) (Utilities|Array|MakeArray "/Game/Mods/Mercury/ModSettings") true)
  (bind _outassetdata (Class|AssetRegistry|GetAssets (Class|AssetRegistryHelpers|GetAssetRegistry) (Utilities|MakeARFilter 0 (.packagepaths _filter) 0 (.classnames _filter) 0 (.brecursivepaths _filter) (.brecursiveclasses _filter))))
  (bind _output_get (LocalVariables|SetOut%20Asset%20Data _outassetdata))
  (for _array_element _output_get
    (bind _returnvalue (Utilities|LoadAssetBlocking (Class|KismetSystemLibrary|ToSoftObjRef(SoftObjPath) (Utilities|MakeSoftObjectPath (Utilities|String|Replace (Class|KismetSystemLibrary|GetPathName (Class|AssetRegistryHelpers|GetAsset _array_element)) "." ".Default__")))))
    (bind _aspda_mod_settings (Utilities|Casting|CastToPDA_ModSettings _returnvalue))
    (if (not (Utilities|Array|IsEmpty (Variables|/Game/Mods/Mercury/Blueprints/PDA_ModSettings.PDA_ModSettings_C|GetModName _aspda_mod_settings)))
      (Utilities|Array|AddUnique (Variables|ModSettings|GetModSettingDataAssets) _aspda_mod_settings)
      (Variables|ModSettings|SetModSettingsLoaded true))))

(fn AddOutdatedPaktoDM
  (params (PakName :type String))
  (Default|AddPaktoContainer (Variables|/Game/Mods/Mercury/UI/Widgets/WBP_UI_ModManager_ModStack.WBP_UI_ModManager_ModStack_C|GetWBP_UI_ModManager_DownloadManager (Variables|Default|GetModStack)) (Utilities|Text|ToText(String) PakName)))

(fn UpdateModDownloadProgress
  (params (PakName :type String) (Progress :type Float%20%28single-precision%29))
  (bind _modstack (Variables|Default|GetModStack)
    (:then
      (for _array_element (Class|PanelWidget|GetAllChildren (Variables|/Game/Mods/Mercury/UI/Widgets/DownloadManager/WBP_UI_ModManager_DownloadManager.WBP_UI_ModManager_DownloadManager_C|GetPakModsContainer (Variables|/Game/Mods/Mercury/UI/Widgets/WBP_UI_ModManager_ModStack.WBP_UI_ModManager_ModStack_C|GetWBP_UI_ModManager_DownloadManager _modstack)))
        (bind _aswbp_ui_mod_manager_base_download (Utilities|Casting|CastToWBP_UI_ModManager_BASE_Download _array_element))
        (if (Utilities|Enum|Equal(Enum) (Variables|/Game/Mods/Mercury/UI/Widgets/DownloadManager/WBP_UI_ModManager_BASE_Download.WBP_UI_ModManager_BASE_Download_C|GetPakName _aswbp_ui_mod_manager_base_download) PakName)
          (Variables|/Game/Mods/Mercury/UI/Widgets/DownloadManager/WBP_UI_ModManager_BASE_Download.WBP_UI_ModManager_BASE_Download_C|SetDownloadProgressValue _aswbp_ui_mod_manager_base_download Progress))))
    (:else)))

(fn UpdateAllMods)