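; Mod manager Blueprint that links the mod manager UI to mod update and pak load order data.
; Tick syncs the notifier's outdated-mod count and finds the ModStack widget, giving it a back-reference.
; Helper functions add paks to the load order widget and read its entries back into PakStrings.
; RefreshLoadOrder is an empty stub hooked in C++; CheckForUpdates, called shortly after BeginPlay, is also empty here.
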(event EventBeginPlay
  (Utilities|FlowControl|Delay 0.5)
  (CallFunction|CheckforUpdates))

(event EventTick
  (params (DeltaSeconds :type Float%20%28single-precision%29))
  (Utilities|FlowControl|Sequence
    (:then_0
      (if (not (Utilities|Enum|Equal(Enum) (Class|RichTextBlock|GetText (Variables|/Game/Mods/_NadzMods/ModManager/Widgets/WBP_UI_ModManager_MainMenuNotifier.WBP_UI_ModManager_MainMenuNotifier_C|GetUpdatesCountText (Variables|Default|GetModManagerNotifier))) (Utilities|Text|ToText(Integer) (Variables|Default|GetOutdatedMods))))
        (CallFunction|UpdateOutdatedModCount)))
    (:then_1
      (Variables|Default|GetModStack
        (:then)
        (:else
          (bind _foundwidgets (Widget|GetAllWidgetsOfClass "/Game/Mods/_NadzMods/ModManager/Widgets/WBP_UI_ModManager_ModStack.WBP_UI_ModManager_ModStack_C" false))
          (for _array_element _foundwidgets
            (bind _output_get (Variables|Default|SetModStack _array_element))
            (Variables|/Game/Mods/_NadzMods/ModManager/Widgets/WBP_UI_ModManager_ModStack.WBP_UI_ModManager_ModStack_C|SetModManager _output_get self)
            (Variables|Default|SetHasModStack true)))))))

(fn ConstructionScript
  (|CallParentFunction))

(fn CheckforUpdates)

(fn UpdateOutdatedModCount
  (bind _outdatedmods (Variables|Default|GetOutdatedMods))
  (Default|UpdateModText (Variables|Default|GetModManagerNotifier) (Utilities|Text|ToText(Integer) _outdatedmods) _outdatedmods))

(fn AddPaktoLoadOrderList
  (params (PakName :type String))
  (Default|AddPaktoContainer (Variables|/Game/Mods/_NadzMods/ModManager/Widgets/WBP_UI_ModManager_ModStack.WBP_UI_ModManager_ModStack_C|GetWBP_UI_ModManager_LoadOrder (Variables|Default|GetModStack)) (Utilities|Text|ToText(String) PakName)))

(fn RefreshLoadOrder
  ;[1 1 1] Hooked in c++
)

(fn GetandSetPakStringsArray
  (bind _modstack (Variables|Default|GetModStack)
    (:then
      (Utilities|Array|Clear (Variables|Default|GetPakStrings))
      (for _array_element (Class|PanelWidget|GetAllChildren (Variables|/Game/Mods/_NadzMods/ModManager/Widgets/LoadOrder/WBP_UI_ModManager_LoadOrder.WBP_UI_ModManager_LoadOrder_C|GetPakModsContainer (Variables|/Game/Mods/_NadzMods/ModManager/Widgets/WBP_UI_ModManager_ModStack.WBP_UI_ModManager_ModStack_C|GetWBP_UI_ModManager_LoadOrder _modstack)))
        (bind _aswbp_ui_mod_manager_base_pak_mod (Utilities|Casting|CastToWBP_UI_ModManager_BASE_PakMod _array_element))
        (Utilities|Array|Add (Variables|Default|GetPakStrings) (Utilities|String|ToString(Text) (Class|TextBlock|GetText (Variables|/Game/Mods/_NadzMods/ModManager/Widgets/LoadOrder/WBP_UI_ModManager_BASE_PakMod.WBP_UI_ModManager_BASE_PakMod_C|GetText_ModName_1 _aswbp_ui_mod_manager_base_pak_mod))))))
    (:else)))